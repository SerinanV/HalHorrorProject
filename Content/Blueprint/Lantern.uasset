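; Lantern is a world pickup actor that the first-person player collects by interacting with it.
; Overlapping its InteractionCollision stores the character, enables input on the actor and shows a Japanese "press E to pick up" HUD prompt.
; Leaving the collision disables input and hides the prompt.
; Either the Lantern or Interact input action calls PickUpLantern on the stored character, then destroys the actor.
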(event `self.ReceiveBeginPlay`)

(event `self.InteractionCollision.OnComponentBeginOverlap`
  (params (OverlappedComponent :type "PrimitiveComponent Object Reference") (OtherActor :type "Actor Object Reference") (OtherComp :type "PrimitiveComponent Object Reference") (OtherBodyIndex :type Integer) (bFromSweep :type Boolean) (SweepResult :type "HitResult Structure (by ref)"))
  ;[1 1 1] プレイヤーがインタラクトの範囲内に入った場合
  (bind _asfirst_person_character (cast `/Game/FirstPersonBP/Blueprints/FirstPersonCharacter` OtherActor))
  (set `self.PlayerObject` _asfirst_person_character)
  (`self.EnableInput` (`GameplayStatics.GetPlayerController` 0))
  (bind _guidetext (`/Game/Blueprint/Widget/PlayerUiWidget.GuideText` (`/Game/FirstPersonBP/Blueprints/FirstPersonCharacter.HudWidget` _asfirst_person_character)))
  (`Widget.SetVisibility` _guidetext "Visible")
  (`TextBlock.SetText` _guidetext "E キーで拾う"))

(event `self.InteractionCollision.OnComponentEndOverlap`
  (params (OverlappedComponent :type "PrimitiveComponent Object Reference") (OtherActor :type "Actor Object Reference") (OtherComp :type "PrimitiveComponent Object Reference") (OtherBodyIndex :type Integer))
  ;[1 1 1] プレイヤーがインタラクトの範囲内から出た場合
  (bind _asfirst_person_character (cast `/Game/FirstPersonBP/Blueprints/FirstPersonCharacter` OtherActor))
  (`self.DisableInput` (`GameplayStatics.GetPlayerController` 0))
  (`Widget.SetVisibility` (`/Game/Blueprint/Widget/PlayerUiWidget.GuideText` (`/Game/FirstPersonBP/Blueprints/FirstPersonCharacter.HudWidget` _asfirst_person_character)) "Hidden"))

(event `InputAction|Lantern`
  (params (Key :type "Key Structure"))
  ;[1 1 1] ランタンを拾う処理（インタラクト）
  (:`Pressed`
    (bind _asfirst_person_character (cast `/Game/FirstPersonBP/Blueprints/FirstPersonCharacter` (`self.PlayerObject`) :!label _label))
    (`/Game/FirstPersonBP/Blueprints/FirstPersonCharacter.PickUpLantern` _asfirst_person_character)
    (`self.K2_DestroyActor`)))

(event `InputAction|Interact`
  (params (Key :type "Key Structure"))
  ;[1 1 1] ランタンを拾う処理（インタラクト）
  (:`Pressed`
    (goto _label)))

(fn `UserConstructionScript`)