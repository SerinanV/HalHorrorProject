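; Classroom door actor that the first-person player opens and closes with Interact while inside its interaction volume.
; A locked door checks the player's inventory for its matching key, then unlocks or reports being locked via HUD text.
; A FlipFlop plays or reverses a timeline that moves the door mesh; InteractByEvent triggers this directly, skipping lock and movement checks.
; When enabled, the player leaving a second volume makes GameManager switch worlds.
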(event `self.InteractionCollision.OnComponentBeginOverlap`
  (params (OverlappedComponent :type "PrimitiveComponent Object Reference") (OtherActor :type "Actor Object Reference") (OtherComp :type "PrimitiveComponent Object Reference") (OtherBodyIndex :type Integer) (bFromSweep :type Boolean) (SweepResult :type "HitResult Structure (by ref)"))
  ;[1 1 1] ドアの範囲内に入った場合、インタラクトを有効化する
  (cast `/Game/FirstPersonBP/Blueprints/FirstPersonCharacter` OtherActor)
  (`self.EnableInput` (`GameplayStatics.GetPlayerController` 0)))

(event `self.InteractionCollision.OnComponentEndOverlap`
  (params (OverlappedComponent :type "PrimitiveComponent Object Reference") (OtherActor :type "Actor Object Reference") (OtherComp :type "PrimitiveComponent Object Reference") (OtherBodyIndex :type Integer))
  ;[1 1 1] ドアの範囲外に出た場合、インタラクトを無効化する
  (cast `/Game/FirstPersonBP/Blueprints/FirstPersonCharacter` OtherActor)
  (`self.DisableInput` (`GameplayStatics.GetPlayerController` 0)))

(event `InputAction|Interact`
  (params (Key :type "Key Structure"))
  (bind _returnvalue_location (`KismetMathLibrary.BreakTransform` (`SceneComponent.GetRelativeTransform` (`self.DoorModel`))))
  (bind _hudwidget (`/Game/FirstPersonBP/Blueprints/FirstPersonCharacter.HudWidget` (`self.Player`)))
  ;[1 1 1] プレイヤーによるインタラクト
  (:`Pressed`
    (if (`self.IsLocked`)
      ;;[1 1 1] 鍵がかかっている場合
      (bind _canopen (`self.IsAbleToOpen`))
      (if _canopen
        (`/Game/Blueprint/Widget/PlayerUiWidget.ShowGuideText` _hudwidget "鍵を使用した！" 0.0)
        (set `self.IsLocked` false)
        (else
          (`/Game/Blueprint/Widget/PlayerUiWidget.ShowGuideText` _hudwidget "鍵がかかっている…" 0.0)))
      (else
        ;;[1 1 1] 鍵がかかっていない場合
        (if (not (`self.IsMoving`))
          (set `self.IsMoving` true :!label _label)
          (bind _isa (`/Engine/EditorBlueprintResources/StandardMacros.FlipFlop`)
            (:`A`
              (bind (_direction _locationoffset) (`Timeline|ClassroomDoorTimeline` :!label _label_2)
                (:`Update`
                  (`SceneComponent.K2_SetRelativeLocation` (`self.DoorModel`) (`KismetMathLibrary.MakeVector` (.x _locationoffset) (.y _locationoffset) (.z _returnvalue_location)) false false))
                (:`Finished`
                  (set `self.IsOpened` _isa)
                  (set `self.IsMoving` false))))
            (:`B`
              (goto _label_2 :!via `Reverse`))))))))

(event `InteractByEvent`
  ;[1 1 1] イベントによるインタラクト
  (goto _label))

(event `self.WorldSwitchingCollision.OnComponentEndOverlap`
  (params (OverlappedComponent :type "PrimitiveComponent Object Reference") (OtherActor :type "Actor Object Reference") (OtherComp :type "PrimitiveComponent Object Reference") (OtherBodyIndex :type Integer))
  ;[1 1 1] プレイヤーが通過した場合、世界を切り替える（有効化されている場合）
  (if (`self.EnableWorldSwitching`)
    (cast `/Game/FirstPersonBP/Blueprints/FirstPersonCharacter` OtherActor)
    (`/Game/Blueprint/GameManager.SwitchWorld` (`self.GameManager`))))

(fn `IsAbleToOpen`
  (returns (CanOpen :type Boolean))
  (for _array_element (`/Game/FirstPersonBP/Blueprints/FirstPersonCharacter.Inventory` (`self.Player`))
    (bind _askey (cast `/Game/Blueprint/Item/Key` _array_element))
    (if (== _askey (`self.KeyToUnlock`))
      (return true)))
  (return false))

(fn `UserConstructionScript`
  (`parent.UserConstructionScript`))