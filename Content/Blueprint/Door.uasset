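; Interactive sliding door Blueprint that also switches the game world when the player passes through it.
; An interaction volume enables input while the FirstPersonCharacter overlaps it, so Interact can toggle the door.
; A FlipFlop plays a Timeline forward or in reverse to set the mesh's relative location, with IsMoving blocking presses mid-motion.
; A separate trigger volume calls SwitchWorld on the GameManager when the character enters it.
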(event `self.ReceiveBeginPlay`
  ;[1 1 1] 自身の初期座標を変数に格納する
  (set `self.Default Location` (`SceneComponent.K2_GetComponentLocation` (`self.DoorModel`))))

(event `self.InteractionCollision.OnComponentBeginOverlap`
  (params (OverlappedComponent :type "PrimitiveComponent Object Reference") (OtherActor :type "Actor Object Reference") (OtherComp :type "PrimitiveComponent Object Reference") (OtherBodyIndex :type Integer) (bFromSweep :type Boolean) (SweepResult :type "HitResult Structure (by ref)"))
  ;[1 1 1] ドアの範囲内に入った場合、インタラクトを有効化する
  (cast `/Game/FirstPersonBP/Blueprints/FirstPersonCharacter` OtherActor)
  (`self.EnableInput` (`GameplayStatics.GetPlayerController` 0)))

(event `self.InteractionCollision.OnComponentEndOverlap`
  (params (OverlappedComponent :type "PrimitiveComponent Object Reference") (OtherActor :type "Actor Object Reference") (OtherComp :type "PrimitiveComponent Object Reference") (OtherBodyIndex :type Integer))
  ;[1 1 1] ドアの範囲外に出た場合、インタラクトを無効化する
  (cast `/Game/FirstPersonBP/Blueprints/FirstPersonCharacter` OtherActor)
  (`self.DisableInput` (`GameplayStatics.GetPlayerController` 0)))

(event `InputAction|Interact`
  (params (Key :type "Key Structure"))
  ;[1 1 1] インタラクトされた場合、ドアが動いている最中でなければ作動させる
  (:`Pressed`
    (if (not (`self.IsMoving`))
      (set `self.IsMoving` true)
      (bind _isa (`/Engine/EditorBlueprintResources/StandardMacros.FlipFlop`)
        (:`A`
          (bind (_direction _door_location_offset) (`Timeline|Door Timeline` :!via `PlayFromStart` :!label _label)
            (:`Update`
              (`SceneComponent.K2_SetRelativeLocation` (`self.DoorModel`) _door_location_offset false false))
            (:`Finished`
              (set `self.IsOpened` _isa)
              (set `self.IsMoving` false))))
        (:`B`
          (goto _label :!via `ReverseFromEnd`))))))

(event `self.WorldSwitchingCollision.OnComponentBeginOverlap`
  (params (OverlappedComponent :type "PrimitiveComponent Object Reference") (OtherActor :type "Actor Object Reference") (OtherComp :type "PrimitiveComponent Object Reference") (OtherBodyIndex :type Integer) (bFromSweep :type Boolean) (SweepResult :type "HitResult Structure (by ref)"))
  ;[1 1 1] プレイヤーが通過した場合、世界を切り替える（表世界・裏世界）
  (cast `/Game/FirstPersonBP/Blueprints/FirstPersonCharacter` OtherActor)
  (bind _asgame_manager (cast `/Game/Blueprint/GameManager` (`self.GameManager`)))
  (`/Game/Blueprint/GameManager.SwitchWorld` _asgame_manager))

(fn `UserConstructionScript`)