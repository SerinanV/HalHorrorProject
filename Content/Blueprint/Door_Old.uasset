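; Interactable sliding door that can be locked to a specific key and can optionally switch the world when the player passes through.
; An overlap volume toggles player input, and pressing Interact either checks the inventory for the key, showing HUD guide text, or toggles the timeline-driven slide when idle.
; The Interact custom event toggles it directly, skipping lock and movement checks.
; A second volume calls SwitchWorld on the GameManager when enabled.
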(event `self.ReceiveBeginPlay`
  (bind _asfirst_person_character (cast `/Game/FirstPersonBP/Blueprints/FirstPersonCharacter` (`GameplayStatics.GetPlayerCharacter` 0)))
  (set `self.Player` _asfirst_person_character))

(event `self.InteractionCollision.OnComponentBeginOverlap`
  (params (OverlappedComponent :type "PrimitiveComponent Object Reference") (OtherActor :type "Actor Object Reference") (OtherComp :type "PrimitiveComponent Object Reference") (OtherBodyIndex :type Integer) (bFromSweep :type Boolean) (SweepResult :type "HitResult Structure (by ref)"))
  ;[1 1 1] ドアの範囲内に入った場合、インタラクトを有効化する
  (cast `/Game/FirstPersonBP/Blueprints/FirstPersonCharacter` OtherActor)
  (`self.EnableInput` (`GameplayStatics.GetPlayerController` 0)))

(event `self.InteractionCollision.OnComponentEndOverlap`
  (params (OverlappedComponent :type "PrimitiveComponent Object Reference") (OtherActor :type "Actor Object Reference") (OtherComp :type "PrimitiveComponent Object Reference") (OtherBodyIndex :type Integer))
  ;[1 1 1] ドアの範囲外に出た場合、インタラクトを無効化する
  (cast `/Game/FirstPersonBP/Blueprints/FirstPersonCharacter` OtherActor)
  (`self.DisableInput` (`GameplayStatics.GetPlayerController` 0)))

(event `InputAction|Interact`
  (params (Key :type "Key Structure"))
  (bind _returnvalue_location (`KismetMathLibrary.BreakTransform` (`SceneComponent.GetRelativeTransform` (`self.DoorModel`))))
  (bind _hudwidget (`/Game/FirstPersonBP/Blueprints/FirstPersonCharacter.HudWidget` (`self.Player`)))
  ;[1 1 1] インタラクトされた場合、ドアが動いている最中でなければ作動させる
  (:`Pressed`
    (if (`self.IsLocked`)
      (bind _isunlocked (`self.AttemptToOpen`))
      (if _isunlocked
        (set `self.IsLocked` false)
        (`/Game/Blueprint/Widget/PlayerUiWidget.ShowGuideText` _hudwidget "鍵を使用した。" 0.0)
        (else
          (`/Game/Blueprint/Widget/PlayerUiWidget.ShowGuideText` _hudwidget "鍵がかかっている…" 0.0)))
      (elif (not (`self.IsMoving`))
        (set `self.IsMoving` true :!label _label)
        (bind _isa (`/Engine/EditorBlueprintResources/StandardMacros.FlipFlop`)
          (:`A`
            (bind (_direction _door_location_offset) (`Timeline|Door Timeline` :!label _label_2)
              (:`Update`
                (`SceneComponent.K2_SetRelativeLocation` (`self.DoorModel`) (`KismetMathLibrary.MakeVector` (.x _door_location_offset) (.y _door_location_offset) (.z _returnvalue_location)) false false))
              (:`Finished`
                (set `self.IsOpened` _isa)
                (set `self.IsMoving` false))))
          (:`B`
            (goto _label_2 :!via `Reverse`)))))))

(event `Interact`
  ;[1 1 1] インタラクトされた場合、ドアが動いている最中でなければ作動させる
  (goto _label))

(event `self.WorldSwitchingCollision.OnComponentBeginOverlap`
  (params (OverlappedComponent :type "PrimitiveComponent Object Reference") (OtherActor :type "Actor Object Reference") (OtherComp :type "PrimitiveComponent Object Reference") (OtherBodyIndex :type Integer) (bFromSweep :type Boolean) (SweepResult :type "HitResult Structure (by ref)"))
  ;[1 1 1] プレイヤーが通過した場合、世界を切り替える（有効化されている場合）
  (if (`self.EnableWorldSwitching`)
    (cast `/Game/FirstPersonBP/Blueprints/FirstPersonCharacter` OtherActor)
    (bind _asgame_manager (cast `/Game/Blueprint/GameManager` (`self.GameManager`)))
    (`/Game/Blueprint/GameManager.SwitchWorld` _asgame_manager)))

(fn `AttemptToOpen`
  (returns (IsUnlocked :type Boolean))
  (bind _asfirst_person_character (cast `/Game/FirstPersonBP/Blueprints/FirstPersonCharacter` (`GameplayStatics.GetPlayerCharacter` 0)))
  (for _array_element (`/Game/FirstPersonBP/Blueprints/FirstPersonCharacter.Inventory` _asfirst_person_character)
    (bind _askey (cast `/Game/Blueprint/Item/Key` _array_element))
    (if (== _askey (`self.KeyToUnlock`))
      (return true)))
  (return false))

(fn `UserConstructionScript`)