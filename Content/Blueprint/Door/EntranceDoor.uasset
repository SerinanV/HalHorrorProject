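; EntranceDoor is a door Blueprint that the player can try to interact with, only to be told it is locked.
; Overlapping InteractionTrigger with the FirstPersonCharacter enables input on the actor for player 0, and leaving the trigger disables it.
; Pressing Interact while input is enabled shows a Japanese "It's locked…" guide text through the player's HUD widget, with no unlock or opening logic.
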(event `self.ReceiveBeginPlay`
  (`parent.ReceiveBeginPlay`))

(event `self.InteractionTrigger.OnComponentBeginOverlap`
  (params (OverlappedComponent :type "PrimitiveComponent Object Reference") (OtherActor :type "Actor Object Reference") (OtherComp :type "PrimitiveComponent Object Reference") (OtherBodyIndex :type Integer) (bFromSweep :type Boolean) (SweepResult :type "HitResult Structure (by ref)"))
  ;[1 1 1] プレイヤーがドアの範囲内に入った場合、インタラクトを有効化する
  (cast `/Game/FirstPersonBP/Blueprints/FirstPersonCharacter` OtherActor)
  (`self.EnableInput` (`GameplayStatics.GetPlayerController` 0)))

(event `self.InteractionTrigger.OnComponentEndOverlap`
  (params (OverlappedComponent :type "PrimitiveComponent Object Reference") (OtherActor :type "Actor Object Reference") (OtherComp :type "PrimitiveComponent Object Reference") (OtherBodyIndex :type Integer))
  ;[1 1 1] プレイヤーがドアの範囲内から出た場合、インタラクトを無効化する
  (cast `/Game/FirstPersonBP/Blueprints/FirstPersonCharacter` OtherActor)
  (`self.DisableInput` (`GameplayStatics.GetPlayerController` 0)))

(event `InputAction|Interact`
  (params (Key :type "Key Structure"))
  ;[1 1 1] インタラクトされた場合の処理
  (:`Pressed`
    (`/Game/Blueprint/Widget/PlayerUiWidget.ShowGuideText` (`/Game/FirstPersonBP/Blueprints/FirstPersonCharacter.HudWidget` (`self.Player`)) "鍵がかかっている…" 0.0)))

(fn `UserConstructionScript`
  (`parent.UserConstructionScript`))