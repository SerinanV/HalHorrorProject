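; Pickup item actor that the player collects into their inventory by pressing Interact while in range.
; A collision sphere enables and disables input on the item as the first-person character enters and leaves it.
; Interact adds the item to the inventory of the player cached at BeginPlay, shows a timed HUD guide text, and hides the actor rather than destroying it.
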(event `self.ReceiveBeginPlay`
  ;[1 1 1] プレイヤーを変数に格納
  (bind _asfirst_person_character (cast `/Game/FirstPersonBP/Blueprints/FirstPersonCharacter` (`GameplayStatics.GetPlayerCharacter` 0)))
  (set `self.Player` _asfirst_person_character))

(event `self.SphereCollision.OnComponentBeginOverlap`
  (params (OverlappedComponent :type "PrimitiveComponent Object Reference") (OtherActor :type "Actor Object Reference") (OtherComp :type "PrimitiveComponent Object Reference") (OtherBodyIndex :type Integer) (bFromSweep :type Boolean) (SweepResult :type "HitResult Structure (by ref)"))
  ;[1 1 1] プレイヤーがインタラクト範囲に入った場合、入力を有効化する
  (cast `/Game/FirstPersonBP/Blueprints/FirstPersonCharacter` OtherActor)
  (`self.EnableInput` (`GameplayStatics.GetPlayerController` 0)))

(event `self.SphereCollision.OnComponentEndOverlap`
  (params (OverlappedComponent :type "PrimitiveComponent Object Reference") (OtherActor :type "Actor Object Reference") (OtherComp :type "PrimitiveComponent Object Reference") (OtherBodyIndex :type Integer))
  ;[1 1 1] プレイヤーがインタラクト範囲から出た場合、入力を無効化する
  (cast `/Game/FirstPersonBP/Blueprints/FirstPersonCharacter` OtherActor)
  (`self.DisableInput` (`GameplayStatics.GetPlayerController` 0)))

(event `InputAction|Interact`
  (params (Key :type "Key Structure"))
  ;[1 1 1] インタラクトされた場合の処理
  (:`Pressed`
    (`/Game/FirstPersonBP/Blueprints/FirstPersonCharacter.AddItemToInventory` (`self.Player`) self)
    (`self.ShowPickMessage`)
    (`self.SetActorHiddenInGame` true)))

(event `ShowPickMessage`
  ;[1 1 1] 入手した時のテキスト表示
  (`/Game/Blueprint/Widget/PlayerUiWidget.ShowGuideText` (`/Game/FirstPersonBP/Blueprints/FirstPersonCharacter.HudWidget` (`self.Player`)) "" 3.0))

(fn `UserConstructionScript`)