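; Key item Blueprint that tells the player when a key has been picked up.
; Its ShowPickMessage event calls ShowGuideText on the Player's UI widget with a Japanese "Got the key!" message.
; It holds no other active logic: BeginPlay, overlap and Tick are disabled stubs, and the construction script only calls its parent.
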(event `ShowPickMessage`
  ;[1 1 1] 入手した時のテキスト表示
  (`/Game/Blueprint/PlayerUiWidget.ShowGuideText` (`/Game/FirstPersonBP/Blueprints/FirstPersonCharacter.UiWidget` (`self.Player`)) "鍵を手に入れた！" 0.0))

(fn `UserConstructionScript`
  (`parent.UserConstructionScript`))