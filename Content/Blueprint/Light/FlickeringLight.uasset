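; Flickering light Blueprint that blinks a point light on and off at irregular intervals.
; BeginPlay applies the configured intensity and attenuation radius, then starts an endless execution loop.
; A FlipFlop alternates between random delays from separate on and off duration ranges, with a visibility toggle after each delay feeding back into the FlipFlop instead of using Tick.
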(event `self.ReceiveBeginPlay`
  (bind _pointlight (`self.PointLight`))
  (`LightComponent.SetIntensity` _pointlight (`self.IntensityEnergy`))
  (`LocalLightComponent.SetAttenuationRadius` _pointlight (`self.AttenuationRadius`))
  (`/Engine/EditorBlueprintResources/StandardMacros.FlipFlop` :!label _label
    (:`A`
      (`KismetSystemLibrary.RetriggerableDelay` (`KismetMathLibrary.RandomFloatInRange` (`self.MinOnDuration`) (`self.MaxOnDuration`))))
    (:`B`
      (`KismetSystemLibrary.RetriggerableDelay` (`KismetMathLibrary.RandomFloatInRange` (`self.MinOffDuration`) (`self.MaxOffDuration`)))))
  (`SceneComponent.ToggleVisibility` (`self.PointLight`) false)
  (goto _label))

(fn `UserConstructionScript`)