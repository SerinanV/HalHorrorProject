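; Ghost enemy that teleports around the level and hunts the first-person player to trigger a game over.
; While the player is outside the hunt collision, it jumps to a random actor attached to TeleportLocationsParent once the cooldown has elapsed and it is off-screen.
; Inside that range, it chases the player's GameOverGhostDestination only while recently rendered, turning by yaw to face them.
; Its kill collision touching that component activates the game-over ghost and destroys itself.
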(event `self.ReceiveBeginPlay`
  (set `self.PreviousTeleportTime` (`GameplayStatics.GetTimeSeconds`)))

(event `self.ReceiveActorBeginOverlap`
  (params (OtherActor :type "Actor Object Reference")))

(event `self.ReceiveTick`
  (params (DeltaSeconds :type "Float (single-precision)"))
  (bind _returnvalue (`self.WasRecentlyRendered` 0.2))
  (if (`self.IsPlayerInHuntingRange`)
    (if _returnvalue
      ;[1 1 1] プレイヤーが死亡範囲内まで接近し、かつ幽霊がプレイヤーの視界の範囲内にいる場合、プレイヤーを追いかける
      (`self.HuntPlayer`))
    (else
      (bind _elapsedtime (`self.GetElapsedTimeSinceTeleport`))
      (if (>= _elapsedtime (`self.TeleportCooldown`))
        (if (not _returnvalue)
          (`self.TeleportToRandomLocation`))))))

(event `self.KillPlayerCollision.OnComponentBeginOverlap`
  (params (OverlappedComponent :type "PrimitiveComponent Object Reference") (OtherActor :type "Actor Object Reference") (OtherComp :type "PrimitiveComponent Object Reference") (OtherBodyIndex :type Integer) (bFromSweep :type Boolean) (SweepResult :type "HitResult Structure (by ref)"))
  ;[1 1 1] プレイヤーを殺せる範囲まで接近した場合、プレイヤーを殺す
  (bind _asfirst_person_character (cast `/Game/FirstPersonBP/Blueprints/FirstPersonCharacter` OtherActor))
  (if (== (`/Game/FirstPersonBP/Blueprints/FirstPersonCharacter.GameOverGhostDestination` _asfirst_person_character) OtherComp)
    (`/Game/FirstPersonBP/Blueprints/FirstPersonCharacter.ActivateGameOverGhost` _asfirst_person_character)
    (`self.K2_DestroyActor`)))

(event `HuntPlayer`
  (bind _returnvalue (`GameplayStatics.GetPlayerCharacter` 0))
  (bind (_returnvalue_roll _returnvalue_pitch _returnvalue_yaw) (`KismetMathLibrary.BreakRotator` (`KismetMathLibrary.FindLookAtRotation` (`self.K2_GetActorLocation`) (`self.K2_GetActorLocation` _returnvalue))))
  ;[1 1 1] プレイヤーを追いかける処理（プレイヤーを殺すフラグが立っている場合）
  (bind _asfirst_person_character (cast `/Game/FirstPersonBP/Blueprints/FirstPersonCharacter` _returnvalue))
  (`AIBlueprintHelperLibrary.SimpleMoveToLocation` (`self.GetController`) (`SceneComponent.K2_GetComponentLocation` (`/Game/FirstPersonBP/Blueprints/FirstPersonCharacter.GameOverGhostDestination` _asfirst_person_character)))
  (`self.K2_SetActorRotation` (`KismetMathLibrary.MakeRotator` 0.0 0.0 _returnvalue_yaw) true))

(event `TeleportToRandomLocation`
  (bind _outactors (`self.GetAttachedActors` (`self.TeleportLocationsParent`)))
  ;[1 1 1] ランダムなテレポート地点へテレポートする
  (`self.K2_SetActorLocation` (`self.K2_GetActorLocation` (`|GetArrayItem` _outactors (`KismetMathLibrary.RandomIntegerInRange` 0 (- (`KismetArrayLibrary.Array_Length` _outactors) 1)))))
  (set `self.PreviousTeleportTime` (`GameplayStatics.GetTimeSeconds`)))

(event `self.HuntPlayerCollision.OnComponentBeginOverlap`
  (params (OverlappedComponent :type "PrimitiveComponent Object Reference") (OtherActor :type "Actor Object Reference") (OtherComp :type "PrimitiveComponent Object Reference") (OtherBodyIndex :type Integer) (bFromSweep :type Boolean) (SweepResult :type "HitResult Structure (by ref)"))
  ;[1 1 1] プレイヤーが死亡範囲内に入った場合、プレイヤーを殺すフラグを立てる
  (cast `/Game/FirstPersonBP/Blueprints/FirstPersonCharacter` OtherActor)
  (set `self.IsPlayerInHuntingRange` true))

(event `self.HuntPlayerCollision.OnComponentEndOverlap`
  (params (OverlappedComponent :type "PrimitiveComponent Object Reference") (OtherActor :type "Actor Object Reference") (OtherComp :type "PrimitiveComponent Object Reference") (OtherBodyIndex :type Integer))
  ;[1 1 1] プレイヤーが死亡範囲内から出た場合、プレイヤーを殺すフラグを消す
  (cast `/Game/FirstPersonBP/Blueprints/FirstPersonCharacter` OtherActor)
  (set `self.IsPlayerInHuntingRange` false))

(fn `GetElapsedTimeSinceTeleport`
  (returns (ElapsedTime :type "Float (double-precision)"))
  (return (- (`GameplayStatics.GetTimeSeconds`) (`self.PreviousTeleportTime`))))

(fn `UserConstructionScript`)